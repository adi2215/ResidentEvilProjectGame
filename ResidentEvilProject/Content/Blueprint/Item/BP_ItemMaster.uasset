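; BP_ItemMaster is a world pickup actor, apparently the base for items, that adds itself to the player's inventory on touch.
; On BeginPlay it uses its ItemID as the row name to load its data struct from DT_InventoryData.
; When BP_ThirdPersonCharacter overlaps its sphere, it passes ItemID and Amount to the character's inventory component, posts a HUD item note, and destroys itself.
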(event `self.ReceiveBeginPlay`
  (`self.Initialize Item Data Structure`))

(event `self.Sphere.OnComponentBeginOverlap`
  (params (OverlappedComponent :type "PrimitiveComponent Object Reference") (OtherActor :type "Actor Object Reference") (OtherComp :type "PrimitiveComponent Object Reference") (OtherBodyIndex :type Integer) (bFromSweep :type Boolean) (SweepResult :type "HitResult Structure (by ref)"))
  (bind _asbp_third_person_character (cast `/Game/ThirdPerson/Blueprints/BP_ThirdPersonCharacter` OtherActor))
  (`/Game/Blueprint/Inventory/BPAC_InventoryComponent.AddItem` (`/Game/ThirdPerson/Blueprints/BP_ThirdPersonCharacter.BPAC_InventoryComponent` _asbp_third_person_character) (`self.ItemID`) (`self.Amount`))
  (if true
    (`/Game/Blueprint/UI/HUDPLayer.AddItemNotef` (`/Game/ThirdPerson/Blueprints/BP_ThirdPersonCharacter.HUDRef` _asbp_third_person_character) (`self.ItemDataStruct`) (`self.Amount`))
    (`self.K2_DestroyActor`)))

(fn `Initialize Item Data Structure`
  (bind _returnvalue (`|GetDataTableRow` "/Game/Blueprint/Item/DT_InventoryData.DT_InventoryData" (`KismetStringLibrary.Conv_StringToName` (`self.ItemID`)))
    (:`then`
      (set `self.ItemDataStruct` _returnvalue))))

(fn `UserConstructionScript`)