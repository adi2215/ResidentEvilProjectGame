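; BP_MasterClassObj is a master interactable object that shows a widget when the player character is nearby.
; The widget starts hidden, and Sphere overlap events toggle its visibility for a BP_ThirdPersonCharacter that has an InteractionComponent.
; Leaving the sphere also prints a debug message.
; InteractFunc only checks for the InteractionComponent and performs no action.
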(event `self.ReceiveBeginPlay`
  (`SceneComponent.SetVisibility` (`self.Widget`) false false))

(event `/Game/Blueprint/Interaction/BP_Interact.InteractFunc`
  (if (`KismetSystemLibrary.IsValid` (`self.GetComponentByClass` (stale `self.Sphere.OnComponentBeginOverlap` OtherActor) "/Game/Blueprint/Interaction/InteractionComponent.InteractionComponent_C"))
    _))

(event `self.Sphere.OnComponentBeginOverlap`
  (params (OverlappedComponent :type "PrimitiveComponent Object Reference") (OtherActor :type "Actor Object Reference") (OtherComp :type "PrimitiveComponent Object Reference") (OtherBodyIndex :type Integer) (bFromSweep :type Boolean) (SweepResult :type "HitResult Structure (by ref)"))
  (cast `/Game/ThirdPerson/Blueprints/BP_ThirdPersonCharacter` OtherActor)
  (if (`KismetSystemLibrary.IsValid` (`self.GetComponentByClass` OtherActor "/Game/Blueprint/Interaction/InteractionComponent.InteractionComponent_C"))
    (`SceneComponent.SetVisibility` (`self.Widget`) true false)))

(event `self.Sphere.OnComponentEndOverlap`
  (params (OverlappedComponent :type "PrimitiveComponent Object Reference") (OtherActor :type "Actor Object Reference") (OtherComp :type "PrimitiveComponent Object Reference") (OtherBodyIndex :type Integer))
  (cast `/Game/ThirdPerson/Blueprints/BP_ThirdPersonCharacter` OtherActor)
  (if (`KismetSystemLibrary.IsValid` (`self.GetComponentByClass` OtherActor "/Game/Blueprint/Interaction/InteractionComponent.InteractionComponent_C"))
    (`SceneComponent.SetVisibility` (`self.Widget`) false false)
    (`KismetSystemLibrary.PrintText` "Dissapear")))

(fn `UserConstructionScript`)