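; BP_Node1 is an interactable object, apparently a readable note, that toggles an animated display on the character's HUD and pauses the game.
; Its NewFunction event, gated by CanPressE, prints a debug string and flips the Opened state.
; Opening plays the HUD widget animation forward and pauses the game.
; Closing unpauses, plays the same animation in reverse and re-enables CanInteract.
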(event `self.NewFunction`
  (bind _note (`self.Note`))
  (bind _note_2 (`self.Note`))
  (if (`self.CanPressE`)
    (`KismetSystemLibrary.PrintString` "Hello")
    (set `self.CanInteract` false)
    (set `self.Note` (`/Game/Blueprints/CBP_SandboxCharacter.HUD` (`self.Character`)))
    (if (`self.Opened`)
      (set `self.Opened` false)
      (`GameplayStatics.SetGamePaused` false)
      (`UserWidget.PlayAnimation` _note (`/Game/Blueprints/UI/AmmoNumber.dwdwd` _note) 0.0 1 "Reverse" 1.5 false)
      (set `self.CanInteract` true)
      (else
        (set `self.Opened` true)
        (`UserWidget.PlayAnimation` _note_2 (`/Game/Blueprints/UI/AmmoNumber.dwdwd` _note_2) 0.0 1 "Forward" 1.5 false)
        (`GameplayStatics.SetGamePaused` true)
        (set `self.CanInteract` false)))))

(fn `UserConstructionScript`
  (`parent.UserConstructionScript`))