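; BP_Door2 is an interactable door that the player can open and close only while the third-person character's WeaponCard check passes.
; A sphere overlap caches the character and shows or hides a prompt widget for actors with an InteractionComponent.
; InteractFunc toggles the Opened flag and plays or reverses a timeline that lerps the mesh's yaw 90 degrees from StartingRot.
; Without the card, a second widget appears briefly.
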(event `self.ReceiveBeginPlay`
  (`SceneComponent.SetVisibility` (`self.Widget1`) false false)
  (`SceneComponent.SetVisibility` (`self.Widget`) false false))

(event `self.InteractFunc`
  (bind (_startingrot_roll _startingrot_pitch _startingrot_yaw) (`KismetMathLibrary.BreakRotator` (`self.StartingRot`)))
  (if (`KismetSystemLibrary.IsValid` (`self.GetComponentByClass` (stale `self.Sphere.OnComponentBeginOverlap` OtherActor) "/Game/Blueprint/Interaction/InteractionComponent.InteractionComponent_C"))
    (if (`/Game/ThirdPerson/Blueprints/BP_ThirdPersonCharacter.Weapon Card` (stale `self.Sphere.OnComponentBeginOverlap` _asbp_third_person_character))
      (if (`self.Opened`)
        (set `self.Opened` false)
        (bind (_direction _alpha) (`Timeline|Шкала времени` :!via `Reverse` :!label _label)
          (:`Update`
            (`SceneComponent.K2_SetRelativeRotation` (`self.ViewAdjustedStaticMeshGizmo`) (`KismetMathLibrary.MakeRotator` _startingrot_roll _startingrot_pitch (`KismetMathLibrary.Lerp` _startingrot_yaw (- _startingrot_yaw 90.0) _alpha)) false false)
            (`KismetSystemLibrary.Delay` 0.2)))
        (else
          (set `self.Opened` true)
          (goto _label :!via `PlayFromStart`)))
      (else
        (`SceneComponent.SetVisibility` (`self.Widget1`) true false)
        (`KismetSystemLibrary.Delay` 3.0)
        (`SceneComponent.SetVisibility` (`self.Widget1`) false false)))))

(event `self.Sphere.OnComponentBeginOverlap`
  (params (OverlappedComponent :type "PrimitiveComponent Object Reference") (OtherActor :type "Actor Object Reference") (OtherComp :type "PrimitiveComponent Object Reference") (OtherBodyIndex :type Integer) (bFromSweep :type Boolean) (SweepResult :type "HitResult Structure (by ref)"))
  (bind _asbp_third_person_character (cast `/Game/ThirdPerson/Blueprints/BP_ThirdPersonCharacter` OtherActor))
  (if (`KismetSystemLibrary.IsValid` (`self.GetComponentByClass` OtherActor "/Game/Blueprint/Interaction/InteractionComponent.InteractionComponent_C"))
    (`SceneComponent.SetVisibility` (`self.Widget`) true false)))

(event `self.Sphere.OnComponentEndOverlap`
  (params (OverlappedComponent :type "PrimitiveComponent Object Reference") (OtherActor :type "Actor Object Reference") (OtherComp :type "PrimitiveComponent Object Reference") (OtherBodyIndex :type Integer))
  (cast `/Game/ThirdPerson/Blueprints/BP_ThirdPersonCharacter` OtherActor)
  (if (`KismetSystemLibrary.IsValid` (`self.GetComponentByClass` OtherActor "/Game/Blueprint/Interaction/InteractionComponent.InteractionComponent_C"))
    (`SceneComponent.SetVisibility` (`self.Widget`) false false)
    (`KismetSystemLibrary.PrintText` "Dissapear")))

(fn `UserConstructionScript`
  (`parent.UserConstructionScript`))