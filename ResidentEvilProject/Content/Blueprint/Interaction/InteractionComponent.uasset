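; An interaction component that tracks interactable overlaps and computes a view ray from the center of the player's screen.
; The overlap event raises or lowers a counter as overlaps begin and end.
; CalculateTrace deprojects the viewport center through the first player controller and returns a start point and an end point a short fixed reach along that direction.
; The file itself performs no trace and does not read the counter.
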(event `OnInteractableOverlap`
  (params (Overlap :type Boolean))
  (set `self.OverlapCounter` (+ (`self.OverlapCounter`) (select `bool` Overlap :`false` -1 :`true` 1))))

(fn `Calculate Trace`
  (returns (WorldLocation :type "Vector Structure") (ReturnValue :type "Vector Structure"))
  (bind _returnvalue (`GameplayStatics.GetPlayerController` 0))
  (bind (_sizex _sizey) (`PlayerController.GetViewportSize` _returnvalue))
  (bind (_worldlocation _worlddirection) (`PlayerController.DeprojectScreenPositionToWorld` _returnvalue (`KismetMathLibrary.Conv_IntToDouble` (/ _sizex 2)) (`KismetMathLibrary.Conv_IntToDouble` (/ _sizey 2))))
  (return _worldlocation (+ _worldlocation (* _worlddirection 250.0))))